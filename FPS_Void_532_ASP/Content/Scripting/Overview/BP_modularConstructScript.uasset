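; Modular wall actor that builds a row of repeated mesh sections from a configurable section count.
; The Construction Script adds one Instanced Static Mesh instance per section, spaced 400 units apart along local X.
; It applies NewMaterial to the component's first material slot within the same loop.
; The event graph holds only disabled placeholder events, so there is no runtime logic.
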(event EventBeginPlay)

(event Collision|EventActorBeginOverlap
  (params (OtherActor :type Actor%20Object%20Reference)))

(event EventTick
  (params (DeltaSeconds :type Float%20%28single-precision%29)))

(fn ConstructionScript
  ;[0.1562 0.1562 0.1562 0.298] Modular wall (expands wall via script and tiles materials)
  (for _index (range 0 (- (Variables|Default|GetNumSections) 1))
    (Components|InstancedStaticMesh|AddInstance (Variables|Default|GetInstancedStaticMesh) (Math|Transform|MakeTransform (Math|Vector|MakeVector (Math|Conversions|ToFloat(Integer) (* _index 400)) 0.0 0.0)) false)
    (Rendering|Material|SetMaterial (Variables|Default|GetInstancedStaticMesh) 0 (Variables|Default|GetNewMaterial))))